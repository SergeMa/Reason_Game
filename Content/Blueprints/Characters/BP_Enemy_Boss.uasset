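; Boss enemy Blueprint that triggers stage transitions as the boss loses health.
; On BeginPlay it caches itself as an Enemy_Boss_Character via the movement component's owner, along with its max health.
; Tick calls HandleStageTransition, defined outside these graphs, whenever the health ratio is at or below the current threshold.
; ChangeStage lowers that threshold from half to a quarter, then to a negative value after the second stage change.
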(event `self.ReceiveBeginPlay`
  (bind _asenemy_boss_character (cast `Enemy_Boss_Character` (`PawnMovementComponent.GetPawnOwner` (`self.CharacterMovement`))))
  (set `self.Boss character` _asenemy_boss_character)
  (set `self.Max Health` (`Character_Base.MaxHealth` (`self.Boss character`)))
  (set `self.Stage switch percentage` 0.5))

(event `self.ReceiveTick`
  (params (DeltaSeconds :type "Float (single-precision)"))
  (if (<= (/ (`Character_Base.Health` (`self.Boss character`)) (`self.Max Health`)) (`self.Stage switch percentage`))
    (`self.HandleStageTransition`)))

(event `self.ChangeStage`
  (params (StageNum :type Integer))
  (switch `int` StageNum
    (:`1`
      (set `self.Stage switch percentage` 0.25))
    (:`2`
      (set `self.Stage switch percentage` -1.0))))

(fn `UserConstructionScript`)